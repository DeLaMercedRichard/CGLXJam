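; Base stat manager for the building system, storing each building stat's min, current and max values in a map keyed by enum.
; SetUpStats removes the first enum entry, re-applies every remaining stat through SetStats, then fires OnStatsSetUp.
; SetStats clamps values for existing keys and optionally calls UpdateStats, while ModifyStat applies non-zero deltas through it.
; UpdateStats and OnStatsSetUp are empty hooks.
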(event `SetUpStats`
  (bind _stats (`self.Stats`))
  (`BlueprintMapLibrary.Map_Remove` _stats "NewEnumerator0")
  (bind _keys (`BlueprintMapLibrary.Map_Keys` _stats))
  (for _array_element _keys
    (`self.SetStats` _array_element (`self.GetStats` _array_element)))
  (`self.OnStatsSetUp`))

(event `OnStatsSetUp`)

(fn `GetStats`
  (params (E_BP_BuildingStats :type "/Game/BuildingSystem/BluePrints/Enums/E_BP_BuildingStats Enum" :default "NewEnumerator0"))
  (returns (CurrentValue :type Integer) (`Stat Value` :type "/Game/BuildingSystem/BluePrints/Enums/F_BP_BuildingStats Structure"))
  (bind _value (`BlueprintMapLibrary.Map_Find` (`self.Stats`) E_BP_BuildingStats))
  (return (`.CurrentValue_5_A6BDD1B643E62EE903F77F9FC5387D7D` (break `/Game/BuildingSystem/BluePrints/Enums/F_BP_BuildingStats` _value)) _value))

(fn `ModifyStat`
  (params (Stat :type "/Game/BuildingSystem/BluePrints/Enums/E_BP_BuildingStats Enum" :default "NewEnumerator0") (By :type Integer))
  (if (!= By 0)
    (`self.SetStats` Stat (+ (`self.GetStats` Stat) By))
    (return)
    (else
      (return))))

(fn `SetStats`
  (params (Stats :type "/Game/BuildingSystem/BluePrints/Enums/E_BP_BuildingStats Enum" :default "NewEnumerator0") (NewValue :type Integer) (DoUpdate :type Boolean :default true))
  (locals (localStat :type "/Game/BuildingSystem/BluePrints/Enums/E_BP_BuildingStats Enum" :default "NewEnumerator0"))
  (bind (_minvalue _currentvalue _maxvalue) (break `/Game/BuildingSystem/BluePrints/Enums/F_BP_BuildingStats` (`.Stat Value` (`self.GetStats` (`local.localStat`)))))
  (bind _output_get (set `local.localStat` Stats))
  (bind _keys (`BlueprintMapLibrary.Map_Keys` (`self.Stats`)))
  (if (`KismetArrayLibrary.Array_Contains` _keys _output_get)
    (`BlueprintMapLibrary.Map_Add` (`self.Stats`) (`local.localStat`) (make `/Game/BuildingSystem/BluePrints/Enums/F_BP_BuildingStats` _minvalue (`KismetMathLibrary.Clamp` NewValue _minvalue _maxvalue) _maxvalue))
    (if DoUpdate
      (`self.UpdateStats` (`local.localStat`)))))

(fn `UpdateStats`
  (params (E_Building_Stats :type "/Game/BuildingSystem/BluePrints/Enums/E_BP_BuildingStats Enum" :default "NewEnumerator0")))