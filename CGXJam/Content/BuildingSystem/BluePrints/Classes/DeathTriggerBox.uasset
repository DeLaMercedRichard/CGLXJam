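; DeathTriggerBox is a trigger actor that kills the player on overlap and restarts the current level.
; BeginPlay caches the player character and picks an abyss, splash or spike death sound from its hazard-type booleans.
; When the player overlaps, it plays that sound, sets IsDead on the character and reopens the level by name after a short delay.
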(event `self.ReceiveBeginPlay`
  (bind _returnvalue (`GameplayStatics.GetActorOfClass` (`self.CharacterClassRef`)))
  (set `self.PlayerObjectRef` _returnvalue)
  (if (`self.IsAbyss`)
    (set `self.DeathFX` "/Game/Movies/SFX/sfx_abyssDeath_Cue.sfx_abyssDeath_Cue")
    (elif (`self.IsWater`)
      (set `self.DeathFX` "/Game/Movies/SFX/sfx_splashDeath_Cue.sfx_splashDeath_Cue")
      (elif (`self.IsSpike`)
        (set `self.DeathFX` "/Game/Movies/SFX/sfx_spikeDeath_Cue.sfx_spikeDeath_Cue")))))

(event `self.ReceiveActorBeginOverlap`
  (params (OtherActor :type "Actor Object Reference"))
  ;[1 1 1] If Player
  (bind _returnvalue (`GameplayStatics.GetActorOfClass` (`self.CharacterClassRef`)))
  (if (== OtherActor _returnvalue)
    (set `self.HasDied` true)
    (`GameplayStatics.PlaySoundAtLocation` (`self.DeathFX`) (`self.K2_GetActorLocation` (`self.GetOwner` _returnvalue)) (struct) 1.0 1.0 0.0 null null null)
    (set `/Game/ThirdPersonCPP/Blueprints/ThirdPersonCharacter.isDead` true (`self.PlayerObjectRef`))
    ;[1 1 1] Death
    (`KismetSystemLibrary.Delay` 5.0)
    (bind _returnvalue_2 (`GameplayStatics.GetCurrentLevelName` true))
    (`GameplayStatics.OpenLevel` (`KismetStringLibrary.Conv_StringToName` _returnvalue_2))))

(fn `UserConstructionScript`)