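; BP_PlayerStats is the player's stats manager in the building system, linking stat values to stat bars in the main HUD widget.
; InitializeManager stores the player reference and runs SetUpStats; OnStatsSetUp then initializes a bar for every key in the Stats map.
; UpdateStats pushes a stat's current value to its bar.
; GetBarForStat resolves the bar through the player's MainWidget, returning the same WStatBar for any stat.
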(event `InitializeManager`
  (params (Player :type "/Game/ThirdPersonCPP/Blueprints/ThirdPersonCharacter Object Reference"))
  (set `self.PlayerRef` Player)
  (`self.SetUpStats`))

(event `self.OnStatsSetUp`
  (bind _keys (`BlueprintMapLibrary.Map_Keys` (`self.Stats`)))
  (for _array_element _keys
    (`/Game/BuildingSystem/Widgets/W_StatBar.InitializeBar` (`self.GetBarForStat` _array_element) (`.Stat Value` (`self.GetStats` _array_element)))))

(fn `GetBarForStat`
  (params (Stat :type "/Game/BuildingSystem/BluePrints/Enums/E_BP_BuildingStats Enum" :default "NewEnumerator0"))
  (returns (Bar :type "/Game/BuildingSystem/Widgets/W_StatBar Object Reference"))
  (return (`/Game/BuildingSystem/Widgets/W_Main.W_StatBar` (`/Game/ThirdPersonCPP/Blueprints/ThirdPersonCharacter.MainWidget` (`self.PlayerRef`)))))

(fn `UpdateStats`
  (params (E_Building_Stats :type "/Game/BuildingSystem/BluePrints/Enums/E_BP_BuildingStats Enum" :default "NewEnumerator0"))
  (`/Game/BuildingSystem/Widgets/W_StatBar.UpdateStat` (`self.GetBarForStat` E_Building_Stats) (`self.GetStats` E_Building_Stats)))