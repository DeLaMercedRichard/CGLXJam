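; BP_Master_Tile is a buildable tile for the building system that exposes its resource cost and highlights when selected.
; BeginPlay copies cost, name, icon and material from TileData and applies the material to the mesh.
; ChageMat sets IsSelected; Tick shows a ghost material, clearing the flag after a short delay, otherwise applying a fixed platform material over the data-driven one.
; ReturnValue reports the tile as destroyable with its cost.
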(event `self.ReceiveBeginPlay`
  (bind (_name _icon _tilematerial _resourcecost) (break `/Game/BuildingSystem/Structures/s_TileData` (`self.TileData`)))
  ;[1 1 1] Assign the Resource Cost based on the provided structure used in buildable tiles. Player can access this value to check for possible building
  (set `self.Resource Cost` _resourcecost)
  (set `self.Tile Name` _name)
  (set `self.Tile Icon` _icon)
  (bind _output_get (set `self.Tile Material` _tilematerial))
  (bind _output_get_2 (set `self.Tile Material` _output_get))
  (`PrimitiveComponent.SetMaterial` (`self.TileMesh`) 0 _output_get_2))

(event `self.ReceiveTick`
  (params (DeltaSeconds :type "Float (single-precision)"))
  ;[1 1 1] Change the Material to be transparent if the material is highlighted by thr player. Resets afer the player removes the ray from the object
  (if (`self.IsSelected`)
    (`PrimitiveComponent.SetMaterial` (`self.TileMesh`) 0 "/Game/BuildingSystem/Materials/M_GhostTile.M_GhostTile")
    (`KismetSystemLibrary.Delay` 0.1)
    (set `self.IsSelected` false)
    (else
      (`PrimitiveComponent.SetMaterial` (`self.TileMesh`) 0 "/Game/BuildingSystem/Materials/M_PlayerPlatformFlat.M_PlayerPlatformFlat"))))

(fn `ChageMat`
  (params (NewParam :type Boolean))
  (returns (NewParam1 :type Boolean))
  (bind _output_get (set `self.IsSelected` NewParam))
  (return _output_get))

(fn `ReturnValue`
  (returns (CanDestroy :type Boolean) (Value :type Integer))
  (return true (`self.Resource Cost`)))

(fn `UserConstructionScript`)